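; Base Blueprint for enemy characters, bridging combat events to the AI Blackboard and attack playback.
; SetCombatTarget writes the given target to the controller's Blackboard under a configurable key name, and Attack calls PlayAttack.
; ChangeDirection flips the actor by combining its current rotation with a 180-degree offset.
; Tick only forwards to the parent, and the construction script is empty.
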(event `/Game/BluePrints/Interfaces/BPI_Enemy.SetCombatTarget`
  (params (CombatTarget :type "Actor Object Reference"))
  ; Sets Combat Target on overlap
  (`BlackboardComponent.SetValueAsObject` (`AIBlueprintHelperLibrary.GetBlackboard` (`self.GetController`)) (`self.CombatTargetBBKeyName`) CombatTarget))

(event `/Game/BluePrints/Interfaces/BPI_Enemy.Attack`
  (`self.PlayAttack`))

(event `self.ReceiveTick`
  (params (DeltaSeconds :type "Float (single-precision)"))
  (`parent.ReceiveTick` DeltaSeconds))

(fn `ChangeDirection`
  (`self.K2_SetActorRotation` (`KismetMathLibrary.ComposeRotators` (`self.K2_GetActorRotation`) (struct :`Yaw` 180.0))))

(fn `UserConstructionScript`)