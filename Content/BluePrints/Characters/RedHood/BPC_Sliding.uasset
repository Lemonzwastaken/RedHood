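; Actor component that gives a character a floor slide, with crouching, a forward velocity burst, ignored move input and a looping-tick update.
; Tick pushes downhill by a force derived from the floor normal, caps speed, and ends the slide when slow or airborne.
; Ending restores cached movement settings, then uncrouches via dispatcher, using a timer-driven upward trace to wait for headroom.
; A MetaSound plays during the slide.
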(event `StartSlide`
  (bind _movementcomponent (`self.MovementComponent`))
  ; Start Slide
  (`self.OnStartStopCrouch` true)
  (set `MovementComponent.Velocity` (* (`Actor.GetActorForwardVector` (`self.GetOwner`)) 1000.0) _movementcomponent)
  (set `CharacterMovementComponent.GroundFriction` 0.0 _movementcomponent)
  (set `CharacterMovementComponent.BrakingDecelerationWalking` 500.0 _movementcomponent)
  (`Controller.SetIgnoreMoveInput` (`GameplayStatics.GetPlayerController` 0) true)
  (`self.SetComponentTickEnabled` true)
  (set `self.Sliding` true)
  (bind _returnvalue (`GameplayStatics.CreateSound2D` "/Game/Assets/Sounds/RedHood/Sliding/MS_FloorSliding.MS_FloorSliding" 1.0 1.0 0.5 null false false))
  (bind _output_get (set `self.SlidingSound` _returnvalue))
  (`AudioComponent.Play` _output_get 0.0))

(event `self.ReceiveBeginPlay`
  (`self.StoreEssentialVariables`))

(event `self.ReceiveTick`
  (params (DeltaSeconds :type "Float (single-precision)"))
  (`self.Slide`)
  (`self.StopSlideInAir`))

(event `EndSlide`
  (bind _returnvalue (`Actor.K2_GetActorLocation` (`self.GetOwner`)))
  ; End Slide
  (set `CharacterMovementComponent.GroundFriction` (`self.GroundFriction`) (`self.MovementComponent`))
  (set `CharacterMovementComponent.BrakingDecelerationWalking` (`self.BrakingDecelerationWalking`) (`self.MovementComponent`))
  (set `CharacterMovementComponent.GravityScale` (`self.GravityScale`) (`self.MovementComponent`))
  (set `self.Sliding` false)
  (bind (_outhit _returnvalue_2) (`KismetSystemLibrary.LineTraceSingle` _returnvalue (+ _returnvalue (0.0 0.0 150.0)) "TraceTypeQuery1"))
  (if (not _returnvalue_2)
    (`self.OnStartStopCrouch` false)
    (else
      (`self.AdaptiveCrouchCheck`)))
  (`Controller.ResetIgnoreMoveInput` (`GameplayStatics.GetPlayerController` 0))
  (`self.SetComponentTickEnabled` false)
  (`AudioComponent.Stop` (`self.SlidingSound`)))

(event `AdaptiveCrouchCheck`
  ; Adaptive Crouch Check
  (bind _returnvalue (`KismetSystemLibrary.K2_SetTimerDelegate` (delegate `CrouchCheckLoop`) 0.1 true))
  (set `self.CrouchCheckTimer` _returnvalue))

(event `CrouchCheckLoop`
  (bind _returnvalue (`Actor.K2_GetActorLocation` (`self.GetOwner`)))
  ; Adaptive Crouch Check
  (bind (_outhit _returnvalue_2) (`KismetSystemLibrary.LineTraceSingle` _returnvalue (+ _returnvalue (0.0 0.0 150.0)) "TraceTypeQuery1"))
  (if (not _returnvalue_2)
    (`KismetSystemLibrary.K2_ClearAndInvalidateTimerHandle` (`self.CrouchCheckTimer`))
    (`self.OnStartStopCrouch` false)))

(fn `CheckIfFloorIsSloped`
  (params (Input :type "Vector Structure"))
  (returns (Output :type "Vector Structure"))
  (bind _input (`local.Input`))
  (if (== Input (`KismetMathLibrary.Vector_Up`) :`ErrorTolerance` 0.0001)
    (return (0.0 0.0 0.0))
    (else
      (return (* (`KismetMathLibrary.Normal` (`KismetMathLibrary.Cross_VectorVector` _input (`KismetMathLibrary.Cross_VectorVector` _input (`KismetMathLibrary.Vector_Up`)))) (* (`KismetMathLibrary.FClamp` (- 1.0 (`KismetMathLibrary.Dot_VectorVector` (`local.Input`) (`KismetMathLibrary.Vector_Up`)))) 500000.0))))))

(fn `Slide`
  (bind _movementcomponent (`self.MovementComponent`))
  (bind (_currentfloor_bblockinghit _currentfloor_bwalkablefloor _currentfloor_blinetrace _currentfloor_floordist _currentfloor_linedist _currentfloor_hitresult) (break `FindFloorResult` (`CharacterMovementComponent.CurrentFloor` _movementcomponent)))
  (`CharacterMovementComponent.AddForce` _movementcomponent (`self.CheckIfFloorIsSloped` (`.Normal` (`GameplayStatics.BreakHitResult` _currentfloor_hitresult))))
  (`|ExecutionSequence`
    (:`then_0`
      ; Set Velocity
      (if (> (`KismetMathLibrary.VSize` (`Actor.GetVelocity` (`self.GetOwner`))) 1000.0)
        (set `MovementComponent.Velocity` (* (`KismetMathLibrary.Normal` (`Actor.GetVelocity` (`self.GetOwner`))) 1000.0) (`self.MovementComponent`))))
    (:`then_1`
      (if (< (`KismetMathLibrary.VSize` (`Actor.GetVelocity` (`self.GetOwner`))) 300.0)
        (`self.EndSlide`)))))

(fn `StopSlideInAir`
  (if (`NavMovementComponent.IsFalling` (`self.MovementComponent`))
    (`AudioComponent.Stop` (`self.SlidingSound`))
    (`self.EndSlide`)))

(fn `StoreEssentialVariables`
  (bind _returnvalue (`Actor.GetComponentByClass` (`self.GetOwner`) "/Script/Engine.CharacterMovementComponent"))
  (`/Engine/EditorBlueprintResources/StandardMacros.IsValid` _returnvalue
    (:`Is Valid`
      (bind _output_get (set `self.MovementComponent` _returnvalue))
      (set `self.GroundFriction` (`CharacterMovementComponent.GroundFriction` _output_get))
      (set `self.BrakingDecelerationWalking` (`CharacterMovementComponent.BrakingDecelerationWalking` _output_get))
      (set `self.GravityScale` (`CharacterMovementComponent.GravityScale` _output_get))
      (bind _returnvalue_2 (`GameplayStatics.CreateSound2D` "/Game/Assets/Sounds/RedHood/Sliding/MS_WallSliding.MS_WallSliding" 1.0 1.0 0.0 null))
      (set `self.SlidingSound` _returnvalue_2))))