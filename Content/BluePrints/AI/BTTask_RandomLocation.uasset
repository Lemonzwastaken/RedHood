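; Behavior Tree task that picks a random wander location for the AI-controlled pawn and stores it in a Blackboard vector key.
; GetRandomPoints samples reachable navmesh points within a fixed radius of the pawn, taking X and Z from the result but keeping the pawn's current Y, so the target varies only in the XZ plane.
; The task always finishes successfully, without checking whether a point was found.
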(event `self.ReceiveExecuteAI`
  (params (OwnerController :type "AIController Object Reference") (ControlledPawn :type "Pawn Object Reference"))
  (`BTFunctionLibrary.SetBlackboardValueAsVector` (`self.BBKey_Location`) (`self.GetRandomPoints` ControlledPawn))
  (`self.FinishExecute` true))

(fn `GetRandomPoints`
  (params (ControlledPawn :type "Actor Object Reference"))
  (returns (ReturnValue :type "Vector Structure"))
  (bind _returnvalue (`Actor.K2_GetActorLocation` ControlledPawn))
  (return (`KismetMathLibrary.MakeVector` (.x (`NavigationSystemV1.K2_GetRandomReachablePointInRadius` _returnvalue 2500.0 null null)) (.y _returnvalue) (.z (`NavigationSystemV1.K2_GetRandomReachablePointInRadius` _returnvalue 2500.0 null null)))))